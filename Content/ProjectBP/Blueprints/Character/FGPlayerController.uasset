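; FGPlayerController is a player controller that sets up the game's UI based on the current level.
; On BeginPlay it creates both the HUD and MainMenu widgets and stores references to them.
; In MainMenuMap it shows the main menu with UI-only input and a visible cursor.
; Any other level shows the HUD with game-only input and a hidden cursor.
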(event `self.ReceiveBeginPlay`
  (bind _returnvalue (`|CreateWidget` "/Game/ProjectBP/Blueprints/Utils/HUD.HUD_C"))
  (bind _returnvalue_2 (`|CreateWidget` "/Game/ProjectBP/Blueprints/Utils/MainMenu.MainMenu_C"))
  (bind _output_get (set `self.MainMenuRef` _returnvalue_2))
  (bind _output_get_2 (set `self.HUD_Ref` _returnvalue))
  (bind _returnvalue_3 (`GameplayStatics.GetCurrentLevelName` true))
  (if (`KismetStringLibrary.EqualEqual_StrStr` _returnvalue_3 "MainMenuMap")
    (`UserWidget.AddToViewport` _output_get 0)
    (`WidgetBlueprintLibrary.SetInputMode_UIOnlyEx` self (`self.MainMenuRef`))
    (set `self.bShowMouseCursor` true)
    (else
      (`UserWidget.AddToViewport` _output_get_2 0)
      (`WidgetBlueprintLibrary.SetInputMode_GameOnly` self)
      (set `self.bShowMouseCursor` false))))

(fn `UserConstructionScript`)
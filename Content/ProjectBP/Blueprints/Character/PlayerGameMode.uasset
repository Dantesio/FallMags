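; Game mode that handles autosaving and loading of level progress, points, respawn position and spawned tiles.
; On BeginPlay it loads or creates the autosave, restores points, respawns the player at the last checkpoint and has the TileSpawner regenerate saved tiles outside the main menu.
; SaveGameOptions writes the current state to the slot, while LoadSaveGame opens the saved level via an enum mapped from level names, defaulting to Level_01.
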(event `Save Game Options`
  (params (Position :type "Vector Structure"))
  (bind _savegameref (`self.SaveGameRef`))
  ;[1 1 1] Savegame
  (`|ExecutionSequence`
    (:`then_0`
      (bind _returnvalue (`GameplayStatics.GetCurrentLevelName` true))
      (bind _level (`self.GetLevelEnum` _returnvalue))
      (set `/Game/ProjectBP/Blueprints/Utils/MySaveGame.Saved_Level` _level _savegameref))
    (:`then_1`
      (set `/Game/ProjectBP/Blueprints/Utils/MySaveGame.LastRespawnPoint` Position _savegameref))
    (:`then_2`
      (set `/Game/ProjectBP/Blueprints/Utils/MySaveGame.Points` (`self.CurrentPoints`) _savegameref))
    (:`then_3`
      (set `/Game/ProjectBP/Blueprints/Utils/MySaveGame.AreTilesSaved` true _savegameref))
    (:`then_4`
      (bind _returnvalue_2 (`GameplayStatics.GetActorOfClass` "/Game/ProjectBP/Blueprints/Utils/TileSpawner.TileSpawner_C"))
      (set `/Game/ProjectBP/Blueprints/Utils/MySaveGame.Saved_Tiles` (`/Game/ProjectBP/Blueprints/Utils/TileSpawner.CurrentTiles` _returnvalue_2) _savegameref))
    (:`then_5`
      (`GameplayStatics.SaveGameToSlot` _savegameref "autosave"))))

(event `self.ReceiveBeginPlay`
  ;[1 1 1] Loading on BeginPlay
  (bind _returnvalue (`GameplayStatics.DoesSaveGameExist` "autosave"))
  (if _returnvalue
    (bind _returnvalue_2 (`GameplayStatics.LoadGameFromSlot` "autosave"))
    (bind _asmy_save_game (cast `/Game/ProjectBP/Blueprints/Utils/MySaveGame` _returnvalue_2))
    (bind _output_get (set `self.SaveGameRef` _asmy_save_game))
    (set `self.CurrentPoints` (`/Game/ProjectBP/Blueprints/Utils/MySaveGame.Points` _output_get))
    (bind _asplayer (cast `/Game/ProjectBP/Blueprints/Character/Player` (`GameplayStatics.GetPlayerCharacter` 0)))
    (`/Game/ProjectBP/Blueprints/Character/Player.Respawn_After_Loading_Level` _asplayer (`/Game/ProjectBP/Blueprints/Utils/MySaveGame.LastRespawnPoint` _output_get))
    (bind _returnvalue_3 (`GameplayStatics.GetCurrentLevelName` true))
    (if (`KismetStringLibrary.NotEqual_StrStr` _returnvalue_3 "MainMenuMap")
      (bind _returnvalue_4 (`GameplayStatics.GetActorOfClass` "/Game/ProjectBP/Blueprints/Utils/TileSpawner.TileSpawner_C"))
      (set `/Game/ProjectBP/Blueprints/Utils/TileSpawner.CurrentTiles` (`/Game/ProjectBP/Blueprints/Utils/MySaveGame.Saved_Tiles` _output_get) _returnvalue_4)
      (`/Game/ProjectBP/Blueprints/Utils/TileSpawner.Generate` _returnvalue_4 false))
    (else
      (bind _returnvalue_5 (`GameplayStatics.CreateSaveGameObject` "/Game/ProjectBP/Blueprints/Utils/MySaveGame.MySaveGame_C"))
      (bind _output_get_2 (set `self.SaveGameRef` _returnvalue_5))
      (`GameplayStatics.SaveGameToSlot` _output_get_2 "autosave")
      (bind _returnvalue_6 (`GameplayStatics.GetActorOfClass` "/Game/ProjectBP/Blueprints/Utils/TileSpawner.TileSpawner_C"))
      (`/Game/ProjectBP/Blueprints/Utils/TileSpawner.Generate` _returnvalue_6 false))))

(event `Load SaveGame`
  (bind _returnvalue (`GameplayStatics.DoesSaveGameExist` "autosave"))
  (if _returnvalue
    (bind _returnvalue_2 (`GameplayStatics.LoadGameFromSlot` "autosave"))
    (bind _asmy_save_game (cast `/Game/ProjectBP/Blueprints/Utils/MySaveGame` _returnvalue_2))
    (`GameplayStatics.OpenLevelBySoftObjectPtr` (select `/Game/ProjectBP/Maps/ELevels` (`/Game/ProjectBP/Blueprints/Utils/MySaveGame.Saved_Level` _asmy_save_game) :`NewEnumerator0` "/Game/ProjectBP/Maps/MainMenuMap.MainMenuMap" :`NewEnumerator1` "/Game/ProjectBP/Maps/Levels/Level1/Level_01.Level_01" :`NewEnumerator2` "/Game/ProjectBP/Maps/Levels/Level_02_1.Level_02_1" :`NewEnumerator3` "/Game/ProjectBP/Maps/Levels/Level_03_1.Level_03_1" :!type "World Soft Object Reference") false)
    (else
      (`GameplayStatics.OpenLevelBySoftObjectPtr` "/Game/ProjectBP/Maps/Levels/Level1/Level_01.Level_01"))))

(fn `GetLevelEnum`
  (params (Name :type String))
  (returns (Level :type "/Game/ProjectBP/Maps/ELevels Enum"))
  (return (select `bool` (`KismetStringLibrary.EqualEqual_StrStr` Name "Level_03_1") :`false` (select `bool` (`KismetStringLibrary.EqualEqual_StrStr` Name "Level_02_1") :`false` (select `bool` (`KismetStringLibrary.EqualEqual_StrStr` Name "Level_01") :`false` "NewEnumerator0" :`true` "NewEnumerator1" :!type "/Game/ProjectBP/Maps/ELevels Enum") :`true` "NewEnumerator2") :`true` "NewEnumerator3")))

(fn `UserConstructionScript`)
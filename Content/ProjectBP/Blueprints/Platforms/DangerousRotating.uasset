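; DangerousRotating is a hazard platform Blueprint that knocks the player away on contact and then reloads the saved game.
; When the player overlaps DangerBox, it enables the character's ragdoll control and launches them horizontally outward from the actor's origin.
; After a short delay, it asks PlayerGameMode to load the save, acting as a death and respawn.
; The graph contains no rotation logic despite the asset's name.
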(event `self.DangerBox.OnComponentBeginOverlap`
  (params (OverlappedComponent :type "PrimitiveComponent Object Reference") (OtherActor :type "Actor Object Reference") (OtherComp :type "PrimitiveComponent Object Reference") (OtherBodyIndex :type Integer) (bFromSweep :type Boolean) (SweepResult :type "HitResult Structure (by ref)"))
  (bind _asplayer (cast `/Game/ProjectBP/Blueprints/Character/Player` OtherActor))
  (`/Game/ProjectBP/Blueprints/Character/Player.RagdollControl` _asplayer true)
  (`Character.LaunchCharacter` _asplayer (* (`KismetMathLibrary.Normal` (`KismetMathLibrary.MakeVector` (.x (- (`self.K2_GetActorLocation` _asplayer) (`self.K2_GetActorLocation`))) (.y (- (`self.K2_GetActorLocation` _asplayer) (`self.K2_GetActorLocation`))))) 700.0) false false)
  (`KismetSystemLibrary.Delay` 3.0)
  (bind _asplayer_game_mode (cast `/Game/ProjectBP/Blueprints/Character/PlayerGameMode` (`GameplayStatics.GetGameMode`)))
  (`/Game/ProjectBP/Blueprints/Character/PlayerGameMode.Load SaveGame` _asplayer_game_mode))

(fn `UserConstructionScript`
  (`parent.UserConstructionScript`))
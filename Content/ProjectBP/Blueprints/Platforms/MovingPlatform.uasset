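; MovingPlatform is a platform actor that moves its Platform component between its start location and an offset.
; On BeginPlay it stores the actor location, sets FloatingTimeline's play rate to 10 divided by MovementTime, and plays it.
; Each update sets the world location by lerping toward start plus FinalEndpoint, without sweeping.
; The lerp alpha is multiplied by the actor's X scale, so scaling changes the travel distance.
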(event `self.ReceiveBeginPlay`
  (bind _returnvalue_x (`KismetMathLibrary.BreakVector` (`self.GetActorScale3D`)))
  (`parent.ReceiveBeginPlay`)
  (bind _output_get (set `self.StartEndpoint` (`self.K2_GetActorLocation`)))
  (`TimelineComponent.SetPlayRate` (`self.Floating Timeline`) (/ 10.0 (`self.MovementTime`)))
  (bind (_direction _float) (`Timeline|Floating Timeline`)
    (:`Update`
      (`SceneComponent.K2_SetWorldLocation` (`self.Platform`) (`KismetMathLibrary.VLerp` _output_get (+ _output_get (`self.FinalEndpoint`)) (* _float _returnvalue_x)) false false))))

(fn `UserConstructionScript`
  (`parent.UserConstructionScript`))
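; Rotating platform that nudges an overlapping player outward from its center.
; On BeginPlay it sets its RotatingMovement rate from a scaled RotationRateZYaw variable.
; SphereCollision overlap events open and close a gate on Tick.
; While the gate is open, each tick feeds a scaled horizontal direction away from the platform into the player's CharacterMovement as movement input.
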(event `self.ReceiveTick`
  (params (DeltaSeconds :type "Float (single-precision)"))
  (`parent.ReceiveTick` DeltaSeconds)
  (`/Engine/EditorBlueprintResources/StandardMacros.Gate` true :!label _label
    (:`Exit`
      (bind _asplayer (cast `/Game/ProjectBP/Blueprints/Character/Player` (stale `self.SphereCollision.OnComponentBeginOverlap` OtherActor)))
      (`PawnMovementComponent.AddInputVector` (`Character.CharacterMovement` _asplayer) (* (`KismetMathLibrary.Normal` (`KismetMathLibrary.MakeVector` (.x (- (`self.K2_GetActorLocation` _asplayer) (`self.K2_GetActorLocation`))) (.y (- (`self.K2_GetActorLocation` _asplayer) (`self.K2_GetActorLocation`))))) 0.4) false))))

(event `self.SphereCollision.OnComponentBeginOverlap`
  (params (OverlappedComponent :type "PrimitiveComponent Object Reference") (OtherActor :type "Actor Object Reference") (OtherComp :type "PrimitiveComponent Object Reference") (OtherBodyIndex :type Integer) (bFromSweep :type Boolean) (SweepResult :type "HitResult Structure (by ref)"))
  (goto _label :!via `Open`))

(event `self.SphereCollision.OnComponentEndOverlap`
  (params (OverlappedComponent :type "PrimitiveComponent Object Reference") (OtherActor :type "Actor Object Reference") (OtherComp :type "PrimitiveComponent Object Reference") (OtherBodyIndex :type Integer))
  (goto _label :!via `Close`))

(event `self.ReceiveBeginPlay`
  (`parent.ReceiveBeginPlay`)
  (set `RotatingMovementComponent.RotationRate` (`KismetMathLibrary.MakeRotator` 0.0 0.0 (* (`self.Rotation Rate Z (Yaw)`) 1.5)) (`self.RotatingMovement`)))

(fn `UserConstructionScript`
  (`parent.UserConstructionScript`))
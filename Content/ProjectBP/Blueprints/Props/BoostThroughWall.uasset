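; BoostThroughWall is a pickup that removes collision from passable walls when a Player overlaps its Sphere.
; On overlap it hides the StaticMesh, disables collision on mesh and Sphere, and calls RemoveCollision on every PassableWall found in the level.
; A parallel Delay branch shows the pickup again and restores its collision after ten seconds, so it can be reused.
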(event `self.Sphere.OnComponentBeginOverlap`
  (params (OverlappedComponent :type "PrimitiveComponent Object Reference") (OtherActor :type "Actor Object Reference") (OtherComp :type "PrimitiveComponent Object Reference") (OtherBodyIndex :type Integer) (bFromSweep :type Boolean) (SweepResult :type "HitResult Structure (by ref)"))
  (cast `/Game/ProjectBP/Blueprints/Character/Player` OtherActor)
  (`|ExecutionSequence`
    (:`then_0`
      (`KismetSystemLibrary.Delay` 10.0)
      (`SceneComponent.SetVisibility` (`self.StaticMesh`) true false)
      (`PrimitiveComponent.SetCollisionEnabled` (`self.StaticMesh`) "QueryAndPhysics")
      (`PrimitiveComponent.SetCollisionEnabled` (`self.Sphere`) "QueryAndPhysics"))
    (:`then_1`
      (`SceneComponent.SetVisibility` (`self.StaticMesh`) false false)
      (`PrimitiveComponent.SetCollisionEnabled` (`self.StaticMesh`) "NoCollision")
      (`PrimitiveComponent.SetCollisionEnabled` (`self.Sphere`) "NoCollision")
      (bind _outactors (`GameplayStatics.GetAllActorsOfClass` "/Game/ProjectBP/Blueprints/Props/PassableWall.PassableWall_C"))
      (for _array_element _outactors
        (`/Game/ProjectBP/Blueprints/Props/PassableWall.RemoveCollision` _array_element)))))

(fn `UserConstructionScript`)
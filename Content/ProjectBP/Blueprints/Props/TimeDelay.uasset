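; TimeDelay is a prop that triggers temporary slow motion when the Player overlaps its sphere.
; On overlap it hides its mesh, disables collision, slows global time to a tenth and raises the player's CustomTimeDilation to partly offset it.
; A one-second Delay in the first Sequence branch, stretched by the slowed time, then restores normal time and re-enables the prop for reuse.
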(event `self.Sphere.OnComponentBeginOverlap`
  (params (OverlappedComponent :type "PrimitiveComponent Object Reference") (OtherActor :type "Actor Object Reference") (OtherComp :type "PrimitiveComponent Object Reference") (OtherBodyIndex :type Integer) (bFromSweep :type Boolean) (SweepResult :type "HitResult Structure (by ref)"))
  (cast `/Game/ProjectBP/Blueprints/Character/Player` OtherActor)
  (`|ExecutionSequence`
    (:`then_0`
      (`KismetSystemLibrary.Delay` 1.0)
      (`SceneComponent.SetVisibility` (`self.StaticMesh`) true false)
      (`PrimitiveComponent.SetCollisionEnabled` (`self.StaticMesh`) "QueryAndPhysics")
      (`PrimitiveComponent.SetCollisionEnabled` (`self.Sphere`) "QueryAndPhysics")
      (bind _asplayer (cast `/Game/ProjectBP/Blueprints/Character/Player` (`GameplayStatics.GetPlayerCharacter` 0)))
      (set `Actor.CustomTimeDilation` 1.0 _asplayer)
      (`GameplayStatics.SetGlobalTimeDilation` 1.0))
    (:`then_1`
      (`SceneComponent.SetVisibility` (`self.StaticMesh`) false false)
      (`PrimitiveComponent.SetCollisionEnabled` (`self.StaticMesh`) "NoCollision")
      (`PrimitiveComponent.SetCollisionEnabled` (`self.Sphere`) "NoCollision")
      (bind _asplayer_2 (cast `/Game/ProjectBP/Blueprints/Character/Player` (`GameplayStatics.GetPlayerCharacter` 0)))
      (set `Actor.CustomTimeDilation` 5.0 _asplayer_2)
      (`GameplayStatics.SetGlobalTimeDilation` 0.1))))

(fn `UserConstructionScript`)
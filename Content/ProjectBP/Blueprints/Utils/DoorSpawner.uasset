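; DoorSpawner is a utility Blueprint that spawns a row of three doors at BeginPlay.
; It spaces them along the world Y axis from the DoorsScene component's location, all at half scale.
; One randomly chosen slot gets a GatesPushing actor and the other two get regular Gates, so the odd door's position varies each play.
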(event `self.ReceiveBeginPlay`
  (set `self.Random` (`KismetMathLibrary.RandomIntegerInRange` 0 2))
  (for _index (range 3)
    (set `self.Location` (+ (`KismetMathLibrary.MakeVector` 0.0 (* _index 520.0)) (`SceneComponent.K2_GetComponentLocation` (`self.DoorsScene`))))
    (if (== _index (`self.Random`))
      (`|SpawnActorFromClass` "/Game/ProjectBP/Blueprints/Props/GatesPushing.GatesPushing_C" (`KismetMathLibrary.MakeTransform` (`self.Location`) (struct) (0.5 0.5 0.5)) "Undefined" "OverrideRootScale" null null)
      (else
        (`|SpawnActorFromClass` "/Game/ProjectBP/Blueprints/Props/Gates.Gates_C" (`KismetMathLibrary.MakeTransform` (`self.Location`) (struct) (0.5 0.5 0.5)) "Undefined" "OverrideRootScale" null null)))))

(fn `UserConstructionScript`)
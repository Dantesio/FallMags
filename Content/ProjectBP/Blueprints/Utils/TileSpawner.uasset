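; TileSpawner is an actor that builds a randomized level as a row of tile level instances when its Generate event fires.
; Each step picks one of seven obstacle tiles, re-rolling to avoid repeating the previous one, and loads it at a fixed spacing.
; Checkpoints spawn between tiles, and a transition actor chosen by CheckLevel caps the end.
; The IsLoading inputs are effectively unused, as saved-tile lookup is deprecated and unreachable.
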(event `Generate`
  (params (IsLoading :type Boolean))
  ;[1 1 1] Script to spawn new Tiles
  (for _index (range (`self.LevelLength`))
    (bind _next (`self.GenerateTileNum` IsLoading _index (`self.Next`) 6))
    (set `self.Next` _next)
    (`LevelStreamingDynamic.LoadLevelInstanceBySoftObjectPtr` (select `int` _next :`0` "/Game/ProjectBP/Maps/TIles/Tile01_MovingPlatforms.Tile01_MovingPlatforms" :`1` "/Game/ProjectBP/Maps/TIles/Tile02_RotatingPlatformsRight.Tile02_RotatingPlatformsRight" :`2` "/Game/ProjectBP/Maps/TIles/Tile03_RotatingPlatformsLeft.Tile03_RotatingPlatformsLeft" :`3` "/Game/ProjectBP/Maps/TIles/Tile04_Wall.Tile04_Wall" :`4` "/Game/ProjectBP/Maps/TIles/TIle05_GuessEnter.TIle05_GuessEnter" :`5` "/Game/ProjectBP/Maps/TIles/Tile06_MettingPlatforms.Tile06_MettingPlatforms" :`6` "/Game/ProjectBP/Maps/TIles/Tile07_DangerRotating.Tile07_DangerRotating" :!type "World Soft Object Reference") (+ (`self.K2_GetActorLocation`) (* (`self.DistanseBetweenTiles`) _index)))
    (if (< _index (- (`self.LevelLength`) 1))
      (`|SpawnActorFromClass` "/Game/ProjectBP/Blueprints/Utils/Checkpoint.Checkpoint_C" (`KismetMathLibrary.MakeTransform` (+ (+ (`self.K2_GetActorLocation`) (* (`self.DistanseBetweenTiles`) (+ _index 1))) (0.0 0.0 15.0))) "Undefined" "OverrideRootScale" null null)))
  (`|SpawnActorFromClass` (select `int` (`self.CheckLevel`) :`0` "/Game/ProjectBP/Blueprints/Utils/LevelTransit1-2.LevelTransit1-2_C" :`1` "/Game/ProjectBP/Blueprints/Utils/LevelTransit2-3.LevelTransit2-3_C" :`2` "/Game/ProjectBP/Blueprints/Utils/LevelTransit_Final.LevelTransit_Final_C" :!type "Actor Class Reference") (`KismetMathLibrary.MakeTransform` (+ (`self.K2_GetActorLocation`) (* (`self.DistanseBetweenTiles`) (`self.LevelLength`)))) "Undefined" "OverrideRootScale" null null))

(fn `GenerateTileNum`
  (params (IsLoading :type Boolean) (LoadingIndex :type Integer) (Previous :type Integer) (Max :type Integer))
  (returns (Next :type Integer))
  (locals (Gen :type Integer))
  (bind _output_get (set `local.Gen` (`KismetMathLibrary.RandomIntegerInRange` 0 Max)))
  (while (== _output_get Previous)
    (bind _output_get_2 (set `local.Gen` (`KismetMathLibrary.RandomIntegerInRange` 0 Max))))
  (return _output_get_2))

(fn `UserConstructionScript`)